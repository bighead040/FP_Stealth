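; Patrol route manager that owns an array of BP_Patrol_Target points, each with a wait time and a use-target-rotation flag.
; AddPatrolPoint spawns a target offset from the base with a back-reference and stores it; ClearAllPatrolPoints destroys all targets and empties the array.
; Settings sync both ways: the Construction Script pushes array values onto targets, and UpdateStruct copies a given target's values back into its entry.
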(event EventBeginPlay)

(event Collision|EventActorBeginOverlap
  (params (OtherActor :type Actor%20Object%20Reference)))

(event EventTick
  (params (DeltaSeconds :type Float%20%28single-precision%29)))

(fn ConstructionScript
  (CallFunction|UpdatePatrolPoint))

(fn AddPatrolPoint
  (bind _returnvalue (Transformation|GetActorTransform))
  (bind (_location _rotation _scale) (Math|Transform|BreakTransform _returnvalue))
  (bind _returnvalue_2 (Game|SpawnActorfromClass "/Game/Blueprints/Gameplay/AI_Patrol/BP_Patrol_Target.BP_Patrol_Target_C" (Math|Transform|MakeTransform (+ _location "50.000000,0.000000,0.000000") _rotation _scale) "Undefined" "MultiplyWithRoot" 0 self 0))
  (Utilities|Array|AddUnique (Variables|PatrolSettings|TargetPoints|GetPatrolTargets) (Utilities|Struct|MakeSTRUCT_PatrolPointInfo _returnvalue_2 (Variables|/Game/Blueprints/Gameplay/AI_Patrol/BP_Patrol_Target.BP_Patrol_Target_C|GetUseTargetRotation _returnvalue_2) (Variables|/Game/Blueprints/Gameplay/AI_Patrol/BP_Patrol_Target.BP_Patrol_Target_C|GetWaitTime _returnvalue_2))))

(fn ClearAllPatrolPoints
  (Utilities|FlowControl|Sequence
    (:then_0
      (for _array_element (Variables|PatrolSettings|TargetPoints|GetPatrolTargets)
        (Actor|DestroyActor (.patroltarget _array_element))))
    (:then_1
      (Utilities|Array|Clear (Variables|PatrolSettings|TargetPoints|GetPatrolTargets)))))

(fn UpdatePatrolPoint
  (for _array_element (Variables|PatrolSettings|TargetPoints|GetPatrolTargets)
    (Variables|/Game/Blueprints/Gameplay/AI_Patrol/BP_Patrol_Target.BP_Patrol_Target_C|SetUseTargetRotation (.PatrolTarget (Utilities|Struct|BreakSTRUCT_PatrolPointInfo _array_element)) (.UseTargetRotation (Utilities|Struct|BreakSTRUCT_PatrolPointInfo _array_element)))
    (Variables|/Game/Blueprints/Gameplay/AI_Patrol/BP_Patrol_Target.BP_Patrol_Target_C|SetWaitTime (.PatrolTarget (Utilities|Struct|BreakSTRUCT_PatrolPointInfo _array_element)) (.WaitTime (Utilities|Struct|BreakSTRUCT_PatrolPointInfo _array_element)))))

(fn UpdateStruct
  (params (PatrolTargetRef :type BP%20Patrol%20Target%20Object%20Reference))
  (for (_array_element _array_index) (Variables|PatrolSettings|TargetPoints|GetPatrolTargets)
    (if (== PatrolTargetRef (.PatrolTarget (Utilities|Struct|BreakSTRUCT_PatrolPointInfo _array_element)))
      (Utilities|Array|SetArrayElem (Variables|PatrolSettings|TargetPoints|GetPatrolTargets) _array_index (Utilities|Struct|MakeSTRUCT_PatrolPointInfo (.PatrolTarget (Utilities|Struct|BreakSTRUCT_PatrolPointInfo _array_element)) (Variables|/Game/Blueprints/Gameplay/AI_Patrol/BP_Patrol_Target.BP_Patrol_Target_C|GetUseTargetRotation PatrolTargetRef) (Variables|/Game/Blueprints/Gameplay/AI_Patrol/BP_Patrol_Target.BP_Patrol_Target_C|GetWaitTime PatrolTargetRef)) true))))
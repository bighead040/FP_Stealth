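; Blaster projectile actor that flies forward and damages what it overlaps, tuned differently for player and non-player shooters.
; PlayerIsInstigator picks a green or red laser material, a faster or slower speed, and higher or lower damage.
; Tick moves it by a fixed per-frame offset without sweep or delta time, and capsule overlap applies damage.
; A timer destroys it after a few seconds; hits do not destroy it.
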(event OnComponentBeginOverlap(CapsuleCollision)
  (params (OverlappedComponent :type Primitive%20Component%20Object%20Reference) (OtherActor :type Actor%20Object%20Reference) (OtherComp :type Primitive%20Component%20Object%20Reference) (OtherBodyIndex :type Integer) (bFromSweep :type Boolean) (SweepResult :type Hit%20Result%20Structure%20%28by%20ref%29))
  (Game|Damage|ApplyDamage OtherActor (select (Variables|Default|GetPlayerIsInstigator) 5e+01 35.0) 0 0))

(event Custom|TimerEvent_DestroySelf
  (Actor|DestroyActor))

(event EventBeginPlay
  (Rendering|Material|SetMaterial (Variables|Default|GetLaserMesh) 0 (select (Variables|Default|GetPlayerIsInstigator) "/Game/Materials/westar34/mm_BlasterShot_green.mm_BlasterShot_green" "/Game/Materials/e11Blaster/m_BlasterShot_red.m_BlasterShot_red"))
  (Utilities|Time|SetTimerbyEvent (delegate Custom|TimerEvent_DestroySelf) 5.0))

(event EventTick
  (params (DeltaSeconds :type Float%20%28single-precision%29))
  (Transformation|AddActorWorldOffset (* (Variables|Default|GetForwardVector) (select (Variables|Default|GetPlayerIsInstigator) 4e+01 3e+01))))

(fn ConstructionScript)
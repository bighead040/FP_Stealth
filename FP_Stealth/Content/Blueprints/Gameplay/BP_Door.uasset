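; Sliding door that opens when the player character or an NPC enters its box collision and closes when they leave, if CanBeOpened.
; Overlaps async-load and play the open or close sound, then play or reverse a timeline lerping the mesh between its BeginPlay location and OpenLocation.
; The construction script colours an indicator by CanBeOpened and shows a translucent preview mesh at OpenLocation, with Y locked to zero.
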(event OnComponentBeginOverlap(BoxCollision)
  (params (OverlappedComponent :type Primitive%20Component%20Object%20Reference) (OtherActor :type Actor%20Object%20Reference) (OtherComp :type Primitive%20Component%20Object%20Reference) (OtherBodyIndex :type Integer) (bFromSweep :type Boolean) (SweepResult :type Hit%20Result%20Structure%20%28by%20ref%29))
  (if (Variables|DoorSettings|GetCanBeOpened)
    (Utilities|IsActorValid OtherActor
      (:true
        (bind _object (Utilities|AsyncLoadAsset (Variables|Default|GetSound_Open))
          (:Completed
            (bind _assound_base (Utilities|Casting|CastToSoundBase _object))
            (Audio|PlaySoundatLocation _assound_base (Transformation|GetActorLocation) "0, 0, 0" 0.75 1.0 0.0 "/Game/Sounds/Attenuation/SA_boots.SA_boots" 0 0 0)
            (bind _alpha (Timeline|TL_Door Play)
              (:Update
                (Transformation|SetRelativeLocation (Variables|Default|GetDoorMesh) (Math|Vector|Lerp(Vector) (Variables|Default|GetCloseLocation) (Variables|DoorSettings|GetOpenLocation) _alpha) false false)))))))))

(event OnComponentEndOverlap(BoxCollision)
  (params (OverlappedComponent :type Primitive%20Component%20Object%20Reference) (OtherActor :type Actor%20Object%20Reference) (OtherComp :type Primitive%20Component%20Object%20Reference) (OtherBodyIndex :type Integer))
  (if (Variables|DoorSettings|GetCanBeOpened)
    (Utilities|IsActorValid OtherActor
      (:true
        (bind _object (Utilities|AsyncLoadAsset (Variables|Default|GetSound_Close))
          (:Completed
            (bind _assound_base (Utilities|Casting|CastToSoundBase _object))
            (Audio|PlaySoundatLocation _assound_base (Transformation|GetActorLocation) "0, 0, 0" 0.75 1.0 0.0 "/Game/Sounds/Attenuation/SA_boots.SA_boots" 0 0 0)
            (bind _alpha (Timeline|TL_Door Reverse)
              (:Update
                (Transformation|SetRelativeLocation (Variables|Default|GetDoorMesh) (Math|Vector|Lerp(Vector) (Variables|Default|GetCloseLocation) (Variables|DoorSettings|GetOpenLocation) _alpha) false false)))))))))

(event EventBeginPlay
  (Variables|Default|SetCloseLocation (Variables|/Script/Engine.SceneComponent|GetRelativeLocation (Variables|Default|GetDoorMesh))))

(fn ConstructionScript
  (bind _previewopen (Variables|Default|GetPreviewOpen))
  (|CallParentFunction)
  (Rendering|Material|SetMaterial (Variables|Default|GetOpeningIndicator) 0 (select (Variables|DoorSettings|GetCanBeOpened) "/Game/Materials/DEBUG/mi_DEBUG_emi_green.mi_DEBUG_emi_green" "/Game/Materials/DEBUG/mi_DEBUG_emi_red.mi_DEBUG_emi_red"))
  (Components|StaticMesh|SetStaticMesh _previewopen (Variables|/Script/Engine.StaticMeshComponent|GetStaticMesh (Variables|Default|GetDoorMesh)))
  (Rendering|Material|SetMaterial _previewopen 0 "/Game/Materials/DEBUG/mi_DEBUG_trans_pink.mi_DEBUG_trans_pink")
  (bind _output_get (Variables|DoorSettings|SetOpenLocation (Math|Vector|MakeVector (.x (Variables|DoorSettings|GetOpenLocation)) 0.0 (.z (Variables|DoorSettings|GetOpenLocation)))))
  (Transformation|SetRelativeLocation (Variables|Default|GetPreviewOpen) _output_get false false))
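; BP_NPC_Base is a base Blueprint for NPCs, defining a common set of functions for barks, patrol and attacking.
; PlayBarkSound, Attack and GetPatrolBase are empty stubs, presumably for child classes to override.
; Simple getters and setters expose the attacking state and a flag for whether to play a patrol bark.
; The event graph holds only disabled default events, so the base runs no logic of its own there.
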(event EventBeginPlay
  (|CallParentFunction) ; This node is disabled and will not be called.\nDrag off pins to build functionality.
)

(event Collision|EventActorBeginOverlap
  (params (OtherActor :type Actor%20Object%20Reference))
  (|CallParentFunction OtherActor) ; This node is disabled and will not be called.\nDrag off pins to build functionality.
)

(event EventTick
  (params (DeltaSeconds :type Float%20%28single-precision%29))
  (|CallParentFunction DeltaSeconds) ; This node is disabled and will not be called.\nDrag off pins to build functionality.
)

(fn ConstructionScript
  (|CallParentFunction))

(fn PlayBarkSound
  (params (BarkType :type ENUM_BarkType_NPC_Enemy%20Enum :default "NewEnumerator0")))

(fn GetPatrolBase
  (return 0))

(fn SetShouldPlayPatrolBark
  (params (PlayPatrolBark :type Boolean))
  (Variables|Default|SetShouldPlayPatrolBark PlayPatrolBark))

(fn GetShouldPlayPatrolBark
  (return (Variables|Default|GetShouldPlayPatrolBark)))

(fn Attack)

(fn GetIsAttacking
  (return (Variables|Default|GetIsAttacking)))

(fn SetIsAttacking
  (params (IsAttacking :type Boolean))
  (Variables|Default|SetIsAttacking IsAttacking))
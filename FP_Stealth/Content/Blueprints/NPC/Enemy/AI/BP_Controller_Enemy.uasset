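; Enemy NPC AI controller that starts the BT_NPC_Enemy behavior tree on BeginPlay and prints the result on screen.
; AI Perception updates for player character 0 store the sensed state and write it to the blackboard as BB_PlayerDetectionActivated.
; The same update snapshots the player's location into TargetLocation, both when sensing succeeds and when it is lost.
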(event OnTargetPerceptionUpdated(AIPerception)
  (params (Actor :type Actor%20Object%20Reference) (Stimulus :type AI%20Stimulus%20Structure))
  (bind _returnvalue (Game|GetPlayerCharacter 0))
  (if (== Actor _returnvalue)
    (bind _output_get (Variables|Default|SetPlayerDetectionActivated (.bSuccessfullySensed (Utilities|Struct|BreakAIStimulus Stimulus))))
    (AI|Components|Blackboard|SetValueasBool (AI|GetBlackboard 0) (Utilities|Name|MakeLiteralName "BB_PlayerDetectionActivated") _output_get)
    (AI|Components|Blackboard|SetValueasVector (AI|GetBlackboard 0) (Utilities|Name|MakeLiteralName "TargetLocation") (Transformation|GetActorLocation _returnvalue))))

(event EventBeginPlay
  (bind _returnvalue (AI|RunBehaviorTree "/Game/Blueprints/NPC/Enemy/AI/BT_NPC_Enemy.BT_NPC_Enemy"))
  (Development|PrintString (Utilities|String|ToString(Boolean) _returnvalue) true false "(R=0.609375,G=0.000000,B=0.000000,A=1.000000)" 1e+01))

(fn ConstructionScript)
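; AI controller for enemy NPCs that runs the enemy behavior tree and escalates detection of the player through patrol, suspicious, investigate and alarmed states.
; AI Perception updates start or clear timers that trigger investigation, a close-range alarm after a short delay, or a return to patrol.
; Each state function sets Blackboard keys for the tree and updates the pawn's barks, with walk speed changing for patrol, investigate and alarmed.
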(event OnTargetPerceptionUpdated(AIPerception)
  (params (Actor :type Actor%20Object%20Reference) (Stimulus :type AI%20Stimulus%20Structure))
  (bind (_age _expirationage _strength _stimuluslocation _receiverlocation _tag _bsuccessfullysensed) (Utilities|Struct|BreakAIStimulus Stimulus))
  (bind _returnvalue (Utilities|Name|MakeLiteralName "BB_Alarmed"))
  (bind _returnvalue_2 (AI|GetBlackboard 0))
  (if (== Actor (Variables|Default|GetPlayerCharacterRef))
    (Variables|Default|SetStimulusLocation _stimuluslocation)
    (if _bsuccessfullysensed
      ;[1 0.8407 0.1] See's Player (goes to Suspicious State)
      (CallFunction|SetBehaviorValueSuspicious)
      (bind _returnvalue_3 (Utilities|Time|SetTimerbyEvent (delegate Custom|TimerEvent_StartInvestigate) (Variables|/Game/Blueprints/BP_NPC_Base.BP_NPC_Base_C|GetBaseTimeTillInvestigate (Variables|Default|GetNPCBaseRef))))
      (Variables|Default|SetTimerHandle_StartInvestigate _returnvalue_3)
      ;[1 0.1 0.1] Player is close (goes to Alarmed State)
      (bind _returnvalue_4 (Utilities|Time|SetTimerbyEvent (delegate Custom|TimerEvent_CheckPlayerDistance) 0.25 true))
      (Variables|Default|SetTimerHandle_CheckPlayerDistance _returnvalue_4)
      (else
        ;[0.1 0.25 1] Lost Player Sight (goes to Patrol State)
        (Default|SetIsAttacking (Variables|Default|GetNPCBaseRef) false)
        (if (or (ScalableFloat|GetValueasBool (AI|GetBlackboard 0) (Utilities|Name|MakeLiteralName "BB_Alarmed")) (ScalableFloat|GetValueasBool (AI|GetBlackboard 0) (Utilities|Name|MakeLiteralName "BB_Suspicious")))
          (Utilities|FlowControl|Sequence
            (:then_0
              (if (or (ScalableFloat|GetValueasBool _returnvalue_2 _returnvalue) (ScalableFloat|GetValueasBool (AI|GetBlackboard 0) (Utilities|Name|MakeLiteralName "BB_IsInvestigating")))
                ;;[1 1 1] If npc is alarmed, start investigate
                (AI|Components|Blackboard|SetValueasBool _returnvalue_2 _returnvalue false)
                (CallFunction|StartInvestigate)
                (else
                  ;;[1 1 1] If npc is suspicious, start "Forget Timer"
                  (bind _returnvalue_5 (Utilities|Time|SetTimerbyEvent (delegate Custom|TimerEvent_ResetPlayerDetection) (Variables|/Game/Blueprints/BP_NPC_Base.BP_NPC_Base_C|GetBaseForgetTime (Variables|Default|GetNPCBaseRef))))
                  (Variables|Default|SetTimerHandle_ResetPlayerDetection _returnvalue_5))))
            (:then_1
              (for _array_element (Utilities|Array|MakeArray (Variables|Default|GetTimerHandle_StartInvestigate) (Variables|Default|GetTimerHandle_CheckPlayerDistance) (Variables|Default|GetTimerHandle_Attack))
                (Utilities|Time|ClearandInvalidateTimerbyHandle _array_element)))))))))

(event Custom|TimerEvent_StartInvestigate
  ;[1 0.19 0.1] See's Player longer (goes to Investigate State)
  (CallFunction|SetBehaviourValueInvestigate "NewEnumerator2")
  (Utilities|Time|SetTimerbyEvent (delegate Custom|TimerEvent_StopInvestigate) (Variables|/Game/Blueprints/BP_NPC_Base.BP_NPC_Base_C|GetBaseInvestigateDuration (Variables|Default|GetNPCBaseRef))))

(event Custom|TimerEvent_StopInvestigate
  ;[1 0.19 0.1] See's Player longer (goes to Investigate State)
  (CallFunction|SetBehaviorValuePatrol))

(event Custom|TimerEvent_ResetPlayerDetection
  ;[0.1 0.25 1] Lost Player Sight (goes to Patrol State)
  ;;[1 1 1] If npc is suspicious, start "Forget Timer"
  (CallFunction|SetBehaviorValuePatrol))

(event Custom|TimerEvent_Attack
  ;[1 0.1 0.1] Player is close (goes to Alarmed State)
  (CallFunction|SetBehaviorValueAlarmed))

(event Custom|TimerEvent_CheckPlayerDistance
  ;[1 0.1 0.1] Player is close (goes to Alarmed State)
  (if (<= (Transformation|GetDistanceTo (Variables|Default|GetPlayerCharacterRef) (Pawn|GetControlledPawn)) 5e+02)
    (Utilities|Time|ClearandInvalidateTimerbyHandle (Variables|Default|GetTimerHandle_CheckPlayerDistance))
    (bind _returnvalue (Utilities|Time|SetTimerbyEvent (delegate Custom|TimerEvent_Attack) 0.5))
    (Variables|Default|SetTimerHandle_Attack _returnvalue)))

(event Custom|StartInvestigate
  ;[1 0.19 0.1] See's Player longer (goes to Investigate State)
  (CallFunction|SetBehaviourValueInvestigate "NewEnumerator5")
  (Utilities|Time|SetTimerbyEvent (delegate Custom|TimerEvent_StopInvestigate) (Variables|/Game/Blueprints/BP_NPC_Base.BP_NPC_Base_C|GetBaseInvestigateDuration (Variables|Default|GetNPCBaseRef))))

(event EventBeginPlay
  (Utilities|FlowControl|Sequence
    (:then_0
      (AI|RunBehaviorTree "/Game/AIBehavior/NPC_Enemy/BT_NPC_Enemy.BT_NPC_Enemy"))
    (:then_1
      (bind _asbp_npc_base (Utilities|Casting|CastToBP_NPC_Base (Pawn|GetControlledPawn)))
      (bind _output_get (Variables|Default|SetNPCBaseRef _asbp_npc_base))
      (bind _patrolbaseref (Default|GetPatrolBase _output_get))
      (bind _output_get_2 (Variables|Default|SetPatrolBaseRef _patrolbaseref))
      (AI|Components|Blackboard|SetValueasObject (AI|GetBlackboard 0) (Utilities|Name|MakeLiteralName "BB_PatrolBaseRef") _output_get_2))
    (:then_2
      (bind _output_get_3 (Variables|Default|SetPlayerCharacterRef (Game|GetPlayerCharacter 0)))
      (AI|Components|Blackboard|SetValueasObject (AI|GetBlackboard 0) (Utilities|Name|MakeLiteralName "BB_PlayerCharacter") _output_get_3))))

(fn ConstructionScript)

(fn SetBehaviorValuePatrol
  (Default|SetIsAttacking (Variables|Default|GetNPCBaseRef) false)
  (AI|Components|Blackboard|SetValueasBool (AI|GetBlackboard 0) (Utilities|Name|MakeLiteralName "BB_IsInvestigating") false)
  (AI|Components|Blackboard|SetValueasBool (AI|GetBlackboard 0) (Utilities|Name|MakeLiteralName "BB_Suspicious") false)
  (bind _npcbaseref (Variables|Default|GetNPCBaseRef)
    (:then
      (Variables|/Script/Engine.CharacterMovementComponent|SetMaxWalkSpeed (Variables|/Script/Engine.Character|GetCharacterMovement _npcbaseref) (Variables|/Game/Blueprints/BP_NPC_Base.BP_NPC_Base_C|GetBasePatrolWalkSpeed _npcbaseref))
      (Default|PlayBarkSound _npcbaseref "NewEnumerator4")
      (Default|SetShouldPlayPatrolBark _npcbaseref true))
    (:else)))

(fn SetBehaviorValueSuspicious
  (Default|SetIsAttacking (Variables|Default|GetNPCBaseRef) false)
  (Utilities|Time|ClearandInvalidateTimerbyHandle (Variables|Default|GetTimerHandle_ResetPlayerDetection))
  (AI|Components|Blackboard|SetValueasBool (AI|GetBlackboard 0) (Utilities|Name|MakeLiteralName "BB_Suspicious") true)
  (Class|BlackboardComponent|SetValueasRotator (AI|GetBlackboard 0) (Utilities|Name|MakeLiteralName "BB_TargetRotation") (Math|Rotator|FindLookatRotation (Transformation|GetActorLocation (Pawn|GetControlledPawn)) (Transformation|GetActorLocation (Variables|Default|GetPlayerCharacterRef))))
  (bind _npcbaseref (Variables|Default|GetNPCBaseRef)
    (:then
      (Default|PlayBarkSound _npcbaseref "NewEnumerator1")
      (Default|SetShouldPlayPatrolBark _npcbaseref false))
    (:else)))

(fn SetBehaviourValueInvestigate
  (params (BarkType :type ENUM_BarkType_NPC_Enemy%20Enum :default "NewEnumerator0"))
  (Default|SetIsAttacking (Variables|Default|GetNPCBaseRef) false)
  (AI|Components|Blackboard|SetValueasBool (AI|GetBlackboard 0) (Utilities|Name|MakeLiteralName "BB_Suspicious") true)
  (AI|Components|Blackboard|SetValueasBool (AI|GetBlackboard 0) (Utilities|Name|MakeLiteralName "BB_IsInvestigating") true)
  (AI|Components|Blackboard|SetValueasVector (AI|GetBlackboard 0) (Utilities|Name|MakeLiteralName "BB_TargetLocation") (Variables|Default|GetStimulusLocation))
  (bind _npcbaseref (Variables|Default|GetNPCBaseRef)
    (:then
      (Variables|/Script/Engine.CharacterMovementComponent|SetMaxWalkSpeed (Variables|/Script/Engine.Character|GetCharacterMovement _npcbaseref) (Variables|/Game/Blueprints/BP_NPC_Base.BP_NPC_Base_C|GetBaseSuspiciousWalkSpeed _npcbaseref))
      (Default|PlayBarkSound _npcbaseref BarkType))
    (:else)))

(fn SetBehaviorValueAlarmed
  (Utilities|Time|ClearandInvalidateTimerbyHandle (Variables|Default|GetTimerHandle_StartInvestigate))
  (for _array_element (Utilities|Array|MakeArray (Utilities|Name|MakeLiteralName "BB_IsInvestigating") (Utilities|Name|MakeLiteralName "BB_Suspicious"))
    (AI|Components|Blackboard|SetValueasBool (AI|GetBlackboard 0) _array_element false))
  (AI|Components|Blackboard|SetValueasBool (AI|GetBlackboard 0) (Utilities|Name|MakeLiteralName "BB_Alarmed") true)
  (AI|Components|Blackboard|SetValueasVector (AI|GetBlackboard 0) (Utilities|Name|MakeLiteralName "BB_TargetLocation") (Transformation|GetActorLocation (Variables|Default|GetPlayerCharacterRef)))
  (bind _npcbaseref (Variables|Default|GetNPCBaseRef)
    (:then
      (Variables|/Script/Engine.CharacterMovementComponent|SetMaxWalkSpeed (Variables|/Script/Engine.Character|GetCharacterMovement _npcbaseref) (Variables|/Game/Blueprints/BP_NPC_Base.BP_NPC_Base_C|GetBaseAlarmedWalkSpeed _npcbaseref))
      (Default|PlayBarkSound _npcbaseref "NewEnumerator3")
      (Default|SetShouldPlayPatrolBark _npcbaseref false))
    (:else)))
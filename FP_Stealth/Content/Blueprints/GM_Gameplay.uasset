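; GM_Gameplay is the gameplay game mode, driving mission flow messages and tracking objective completion.
; On BeginPlay it caps the frame rate by console command and shows the mission-begin widget temporarily.
; MissionItemAcquired briefly shows its widget, setting MissionObjectiveComplete only after the delay and removal.
; MissionSuccessful shows a success widget, then pauses the game after a delay, leaving the widget on screen.
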(event Custom|MissionSuccessful
  (bind _returnvalue (UserInterface|CreateWidget "/Game/UI/WBP_MissionSuccessful.WBP_MissionSuccessful_C" (Game|GetPlayerController 0)))
  (UserInterface|Viewport|AddtoViewport _returnvalue 0)
  (Utilities|FlowControl|Delay 5.0)
  (Game|SetGamePaused true))

(event Custom|MissionItemAcquired
  (bind _returnvalue (UserInterface|CreateWidget "/Game/UI/WBP_MissionItemAcquired.WBP_MissionItemAcquired_C" (Game|GetPlayerController 0)))
  (UserInterface|Viewport|AddtoViewport _returnvalue 0)
  (Utilities|FlowControl|Delay 5.0)
  (Widget|RemovefromParent _returnvalue)
  (Variables|Default|SetMissionObjectiveComplete true))

(event Custom|MissionBegin
  (bind _returnvalue (UserInterface|CreateWidget "/Game/UI/WBP_MissionBegin.WBP_MissionBegin_C" (Game|GetPlayerController 0)))
  (UserInterface|Viewport|AddtoViewport _returnvalue 0)
  (Utilities|FlowControl|Delay 5.0)
  (Widget|RemovefromParent _returnvalue))

(event EventBeginPlay
  (Development|ExecuteConsoleCommand "t.maxfps 60" (Game|GetPlayerController 0))
  (CallFunction|MissionBegin))

(fn ConstructionScript)
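; BP_Controller_Enemy is the AI controller for enemy NPCs, linking player perception and patrol data to their behavior tree.
; On BeginPlay it runs BT_NPC_Enemy, then stores the patrol base from its BP_NPC_Base pawn in the blackboard.
; AI Perception updates concerning the player write the sensed state and a look-at rotation toward the player to the blackboard, on both detection and loss.
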(event OnTargetPerceptionUpdated(AIPerception)
  (params (Actor :type Actor%20Object%20Reference) (Stimulus :type AI%20Stimulus%20Structure))
  (bind _returnvalue (Game|GetPlayerCharacter 0))
  (if (== Actor _returnvalue)
    (bind _output_get (Variables|Default|SetPlayerDetectionActivated (.bSuccessfullySensed (Utilities|Struct|BreakAIStimulus Stimulus))))
    (AI|Components|Blackboard|SetValueasBool (AI|GetBlackboard 0) (Utilities|Name|MakeLiteralName "BB_PlayerDetectionActivated") _output_get)
    (Class|BlackboardComponent|SetValueasRotator (AI|GetBlackboard 0) (Utilities|Name|MakeLiteralName "BB_TargetRotation") (Math|Rotator|FindLookatRotation (Transformation|GetActorLocation (Pawn|GetControlledPawn)) (Transformation|GetActorLocation _returnvalue)))))

(event EventBeginPlay
  (Utilities|FlowControl|Sequence
    (:then_0
      (AI|RunBehaviorTree "/Game/AIBehavior/NPC_Enemy/BT_NPC_Enemy.BT_NPC_Enemy"))
    (:then_1
      (bind _asbp_npc_base (Utilities|Casting|CastToBP_NPC_Base (Pawn|GetControlledPawn)))
      (bind _patrolbaseref (Default|GetPatrolBase _asbp_npc_base))
      (bind _output_get (Variables|Default|SetPatrolBaseRef _patrolbaseref))
      (AI|Components|Blackboard|SetValueasObject (AI|GetBlackboard 0) (Utilities|Name|MakeLiteralName "BB_PatrolBaseRef") _output_get))))

(fn ConstructionScript)